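; BP_SirBrain is the floating Sir Brain actor that watches the player and triggers the win condition.
; A timeline started on BeginPlay bobs the Brain component vertically, while Tick smoothly rotates it to face the player pawn with a yaw offset.
; Each timeline update also reads the score from the SirBrain game instance and opens WinLevel once it reaches the threshold to impress the brain.
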(event EventBeginPlay
  (bind _z (Timeline|FloatingEffect Play)
    (:Update
      (Transformation|SetRelativeLocation (Variables|Default|GetBrain) (Math|Vector|MakeVector 0.0 0.0 (+ _z 2.6e+02)) false false)
      ;[1 1 1] On the hub load check if the score is enough to imrpess brain (aka win)
      (bind _assir_brain (Utilities|Casting|CastToSirBrain (Game|GetGameInstance)))
      (bind _score (Default|GetScore _assir_brain))
      (if (>= _score (Variables|/Game/SirBrain.SirBrain_C|GetScoreToImpressBrain _assir_brain))
        (Game|OpenLevel(byName) "WinLevel")))))

(event EventTick
  (params (DeltaSeconds :type Float%20%28single-precision%29))
  (bind _returnvalue (Game|Player|GetPlayerPawn 0))
  (bind _brain (Variables|Default|GetBrain))
  (bind _returnvalue_2 (Transformation|GetActorLocation _returnvalue))
  (bind _returnvalue_3 (Transformation|GetWorldLocation _brain))
  (bind _returnvalue_4 (Math|Rotator|FindLookatRotation _returnvalue_3 _returnvalue_2))
  (Transformation|SetWorldRotation (Variables|Default|GetBrain) (Math|Interpolation|RInterpTo (Transformation|GetWorldRotation _brain) (Math|Rotator|MakeRotator (.roll _returnvalue_4) (.pitch _returnvalue_4) (+ (.yaw _returnvalue_4) -9e+01)) DeltaSeconds 5.0) false false))

(fn ConstructionScript)