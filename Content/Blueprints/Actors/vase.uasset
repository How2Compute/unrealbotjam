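; Vase actor that receives a Shrubbery when one enters its Box trigger.
; On overlap it snaps the shrubbery to the vase's location, stores it as MyShrub and notifies ShrubGamemode through GotShrubbery.
; The emptyvase event makes the stored shrub unpickable, then destroys it after a short delay.
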(event OnComponentBeginOverlap(Box)
  (params (OtherActor :type Actor%20Object%20Reference) (OtherComp :type Primitive%20Component%20Object%20Reference) (OtherBodyIndex :type Integer) (bFromSweep :type Boolean) (SweepResult :type Hit%20Result%20Structure%20%28by%20ref%29))
  (bind _asshrubbery (Utilities|Casting|CastToShrubbery OtherActor))
  (Transformation|SetActorLocation _asshrubbery (Transformation|GetActorLocation) false false)
  (bind _asshrub_gamemode (Utilities|Casting|CastToShrubGamemode (Game|GetGameMode)))
  (Variables|Default|Setmy%20shrub _asshrubbery)
  (Default|GotShrubbery _asshrub_gamemode self))

(event Custom|empty%20vase
  (Utilities|IsValid (Variables|Default|Getmy%20shrub)
    (:Is%20Valid
      (Variables|/Game/Blueprints/Actors/ItemBase.ItemBase_C|Setcanbepicked (Variables|Default|Getmy%20shrub) false)
      (Utilities|FlowControl|Delay 2.0)
      (Actor|DestroyActor (Variables|Default|Getmy%20shrub)))))

(event EventBeginPlay)

(event EventActorBeginOverlap
  (params (OtherActor :type Actor%20Object%20Reference)))

(event EventTick
  (params (DeltaSeconds :type Float%20%28single-precision%29)))

(fn ConstructionScript)