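; Trigger button actor that activates and releases a linked ActorToTrigger through interfaces, based on overlaps with its Box.
; Overlap by an actor implementing canPressButtonInterface sends UseTriggerMessage to the target via canGetTriggeredInterface.
; On end overlap, it calls ExitTrigger on the target only when no Pawns remain in the Box, without checking the leaving actor's interface.
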(event OnComponentBeginOverlap(Box)
  (params (OtherActor :type Actor%20Object%20Reference) (OtherComp :type Primitive%20Component%20Object%20Reference) (OtherBodyIndex :type Integer) (bFromSweep :type Boolean) (SweepResult :type Hit%20Result%20Structure%20%28by%20ref%29))
  (Utilities|Casting|CastTocanPressButtonInterface OtherActor)
  (bind _ascan_get_triggered_interface (Utilities|Casting|CastTocanGetTriggeredInterface (Variables|Default|Getactor%20to%20trigger)))
  (Class|CanGetTriggeredInterface|UseTrigger(Message) (Utilities|ToObject(Interface) _ascan_get_triggered_interface)))

(event OnComponentEndOverlap(Box)
  (params (OtherActor :type Actor%20Object%20Reference) (OtherComp :type Primitive%20Component%20Object%20Reference) (OtherBodyIndex :type Integer))
  (if (== (Utilities|Array|Length (Collision|GetOverlappingActors (Variables|Default|GetBox) "/Script/Engine.Pawn" :!class /Script/Engine.PrimitiveComponent)) 0)
    (bind _ascan_get_triggered_interface (Utilities|Casting|CastTocanGetTriggeredInterface (Variables|Default|Getactor%20to%20trigger)))
    (Default|ExitTrigger _ascan_get_triggered_interface)))

(event EventBeginPlay)

(event EventActorBeginOverlap
  (params (OtherActor :type Actor%20Object%20Reference)))

(event EventTick
  (params (DeltaSeconds :type Float%20%28single-precision%29)))

(fn ConstructionScript)