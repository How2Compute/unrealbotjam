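; Sliding door actor that opens when its trigger is used and closes when the trigger is exited.
; It caches its starting location on BeginPlay, then a timeline linearly moves the whole actor toward that position plus an end offset.
; Closing reverses the same timeline, so the door slides back from wherever it currently is.
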(event Custom|Open%20Door
  (bind _starting_pos (Variables|Default|Getstarting%20pos))
  (bind _alpha (Timeline|SlidingDoor%20Timeline Play)
    (:Update
      (Transformation|SetActorLocation (Math|Interpolation|Ease "Linear" _alpha _starting_pos (+ _starting_pos (Variables|Default|Getend%20pos%20offset))) false false))))

(event Custom|Close%20Door
  (bind _starting_pos (Variables|Default|Getstarting%20pos))
  (bind _alpha (Timeline|SlidingDoor%20Timeline Reverse)
    (:Update
      (Transformation|SetActorLocation (Math|Interpolation|Ease "Linear" _alpha _starting_pos (+ _starting_pos (Variables|Default|Getend%20pos%20offset))) false false))))

(event EventBeginPlay
  (Variables|Default|Setstarting%20pos (Transformation|GetActorLocation)))

(event EventActorBeginOverlap
  (params (OtherActor :type Actor%20Object%20Reference)))

(event EventTick
  (params (DeltaSeconds :type Float%20%28single-precision%29)))

(event EventUseTrigger
  (CallFunction|OpenDoor))

(event EventExitTrigger
  (CallFunction|CloseDoor))

(fn ConstructionScript)