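; SirBrain tracks a score against a score needed to impress the brain and provides a way to unlock doors by ID.
; Accessor functions return both values, and AddScore adds an amount to the current score, with no threshold comparison in this file.
; UnlockDoor searches every BP_Door actor for a matching DoorID, stops the loop at the first match and unlocks that door.
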(fn GetScore
  (return (Variables|Default|GetScore)))

(fn AddScore
  (params (Ammount :type Integer))
  (Variables|Default|SetScore (+ Ammount (Variables|Default|GetScore))))

(fn GetScoretoImpressBrain
  (return (Variables|Default|GetScoreToImpressBrain)))

(fn UnlockDoor
  (params (ID :type Integer))
  (bind _outactors (Actor|GetAllActorsOfClass "/Game/Meshes/BP_Door.BP_Door_C"))
  (bind _array_element (Utilities|Array|ForEachLoopwithBreak _outactors :!label _label)
    (:LoopBody
      (if (== (Variables|/Game/Meshes/BP_Door.BP_Door_C|GetDoorID _array_element) ID)
        (Utilities|FlowControl|Sequence
          (:then_0
            (goto _label Break))
          (:then_1
            (Default|UnlockDoor _array_element)))))))