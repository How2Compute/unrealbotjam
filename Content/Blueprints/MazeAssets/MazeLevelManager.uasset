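; Maze level manager actor that times the player's run and ends the level when an actor overlaps it.
; Tick accumulates elapsed time, which GetTime exposes.
; On overlap it casts the game instance to SirBrain, adds MaxScore divided by a tenth of the time as score, then opens the hub level.
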(event EventBeginPlay)

(event EventActorBeginOverlap
  (params (OtherActor :type Actor%20Object%20Reference))
  (bind _assir_brain (Utilities|Casting|CastToSirBrain (Game|GetGameInstance)))
  (Default|AddScore _assir_brain (Math|Float|Truncate (/ (Math|Conversions|ToFloat(Integer) (Variables|Default|GetMaxScore)) (/ (Variables|Default|GetTime) 1e+01))))
  (Game|OpenLevel(byName) "hub"))

(event EventTick
  (params (DeltaSeconds :type Float%20%28single-precision%29))
  (Variables|Default|SetTime (+ DeltaSeconds (Variables|Default|GetTime))))

(fn ConstructionScript)

(fn GetTime
  (return (Variables|Default|GetTime)))