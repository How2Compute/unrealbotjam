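; MinigameGamemode is the game mode for a minigame, handling player control at startup and creating the HUD.
; On BeginPlay it runs the Set Player Control graph, which casts the player controller to MinigameController, removes control, waits for StartTime, then restores it.
; It also creates the configured HUD widget, adds it to the viewport and keeps a reference to it.
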(event EventBeginPlay
  (Utilities|FlowControl|Sequence
    (:then_0
      (|Setplayercontrol))
    (:then_1
      (bind _returnvalue (UserInterface|CreateWidget (Variables|Default|GetHUD%20type)))
      (UserInterface|Viewport|AddtoViewport _returnvalue 0)
      (Variables|Default|SetHUD%20reference _returnvalue))))

(event EventTick
  (params (DeltaSeconds :type Float%20%28single-precision%29)))

(fn ConstructionScript)