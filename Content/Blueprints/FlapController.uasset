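; FlapController is a player controller for a Flappy Bird-style game that auto-runs the pawn along +X and flaps it upward on Jump.
; BeginPlay caches the FlapGamemode and FlapPlayer, then uses staggered delays to start movement before enabling input and calling the game mode's DoFlyAnim.
; Tick feeds constant movement input, while Jump launches the character with Z override and plays Boop.
; The losecontrol event clears both flags to stop running and flapping.
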(event Custom|lose%20control
  (Variables|Default|Sethascontrol false)
  (Variables|Default|Sethastorun false))

(event EventBeginPlay
  (Utilities|FlowControl|Sequence
    (:then_0
      (|Setgamemodereference))
    (:then_1
      (|setcharreference))
    (:then_2
      (Utilities|FlowControl|Delay 1.0)
      (Variables|Default|Sethastorun true)
      (Utilities|FlowControl|Delay 4.0)
      (Variables|Default|Sethascontrol true)
      (Default|DoFlyAnim (Variables|Default|Getgamemode%20ref)))))

(event EventTick
  (params (DeltaSeconds :type Float%20%28single-precision%29))
  (if (Variables|Default|Gethastorun)
    (Pawn|Input|AddMovementInput (Pawn|GetControlledPawn) "1.000000, 0, 0" 1.0 false)))

(event Input|ActionEvents|InputActionJump
  (params (Key :type Key%20Structure :default "AnyKey"))
  (:Pressed
    (if (Variables|Default|Gethascontrol)
      (Character|LaunchCharacter (Variables|Default|Getchar%20ref) "0, 0,500.000000" false true)
      (Audio|Components|Audio|Play (Variables|Default|Getboop) 0.0))))

(fn ConstructionScript)