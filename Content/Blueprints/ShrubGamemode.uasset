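; Game mode for a shrubbery delivery level that tracks how many shrubs the player has delivered.
; Its gotshrubbery event receives a vase and branches on the delivery count.
; The first delivery has the ShrubHUD request another shrub and empties the vase.
; The second plays the HUD end animation, adds the score to the SirBrain game instance, then returns to the hub level after a short delay.
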(event Custom|got%20shrubbery
  (params (vase :type Vase%20Object%20Reference))
  (Variables|Default|Setvase%20reference vase)
  (bind _asshrub_hud (Utilities|Casting|CastToShrubHUD (Variables|Default|GetHUD%20reference)))
  (switch int (Variables|Default|Getshrubs%20delivered)
    (:0
      (Default|AnotherShrub _asshrub_hud)
      (Math|Integer|IncrementInt (Variables|Default|Getshrubs%20delivered)
        (:%20%20
          (Default|EmptyVase (Variables|Default|Getvase%20reference)))))
    (:1
      (Default|DoEndAnim _asshrub_hud (Variables|Default|Getscore%20to%20add))
      (Math|Integer|IncrementInt (Variables|Default|Getshrubs%20delivered)
        (:%20%20
          (bind _assir_brain (Utilities|Casting|CastToSirBrain (Game|GetGameInstance)))
          (Default|AddScore _assir_brain (Variables|Default|Getscore%20to%20add))
          (Utilities|FlowControl|Delay 4.0)
          (Game|OpenLevel(byName) "hub"))))))

(event EventBeginPlay
  (|CallParentFunction))

(event EventTick
  (params (DeltaSeconds :type Float%20%28single-precision%29)))

(fn ConstructionScript
  (|CallParentFunction))