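; Game mode for the Flap level that relays fly animation requests to the HUD and handles winning.
; The doflyanim event calls DoFlyAnim on the referenced FlapHUD.
; The win event runs once: it shows the HUD end animation with the score, adds that score to the SirBrain game instance, removes control through FlapController, then opens the hub level after a short delay.
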(event Custom|do%20fly%20anim
  (bind _asflap_hud (Utilities|Casting|CastToFlapHUD (Variables|Default|GetHUD%20reference)))
  (Default|DoFlyAnim _asflap_hud))

(event Custom|win
  (Utilities|FlowControl|DoOnce false
    (:Completed
      (bind _asflap_hud (Utilities|Casting|CastToFlapHUD (Variables|Default|GetHUD%20reference)))
      (Default|DoEndAnim _asflap_hud (Variables|Default|Getscoretoaddtobrain))
      (bind _assir_brain (Utilities|Casting|CastToSirBrain (Game|GetGameInstance)))
      (Default|AddScore _assir_brain (Variables|Default|Getscoretoaddtobrain))
      (bind _asflap_controller (Utilities|Casting|CastToFlapController (Game|GetPlayerController 0)))
      (Default|LoseControl _asflap_controller)
      (Utilities|FlowControl|Delay 4.0)
      (Game|OpenLevel(byName) "hub"))))

(event EventBeginPlay
  (|CallParentFunction))

(event EventTick
  (params (DeltaSeconds :type Float%20%28single-precision%29)))

(fn ConstructionScript
  (|CallParentFunction))