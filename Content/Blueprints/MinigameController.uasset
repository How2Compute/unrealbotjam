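; MinigameController is a controller Blueprint that routes player input to the MinigamePlayer pawn in a minigame.
; On BeginPlay it casts the controlled pawn to MinigamePlayer and caches the reference.
; The x and y axes add movement input scaled by InputSpeed, gated by a Hascontrol flag that Losecontrol and Gaincontrol events toggle.
; The action_1 press calls PickUpItem on the player, without checking that flag.
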(event Custom|Gain%20control
  (Variables|Default|Sethascontrol true))

(event Custom|Lose%20control
  (Variables|Default|Sethascontrol false))

(event EventBeginPlay
  (bind _asminigame_player (Utilities|Casting|CastToMinigamePlayer (Pawn|GetControlledPawn)))
  (Variables|Default|SetPlayer%20reference _asminigame_player))

(event EventTick
  (params (DeltaSeconds :type Float%20%28single-precision%29)))

(event Input|ActionEvents|InputActionaction_1
  (params (Key :type Key%20Structure :default "AnyKey"))
  (:Pressed
    (Default|PickUpItem (Variables|Default|GetPlayer%20reference))))

(event Input|AxisEvents|InputAxisx_axis
  (params (AxisValue :type Float%20%28single-precision%29))
  (if (Variables|Default|Gethascontrol)
    (Pawn|Input|AddMovementInput (Variables|Default|GetPlayer%20reference) (Math|Vector|MakeVector (* AxisValue (Variables|Default|GetInput%20speed)) 0.0 0.0) 1.0 false)))

(event Input|AxisEvents|InputAxisy_axis
  (params (AxisValue :type Float%20%28single-precision%29))
  (if (Variables|Default|Gethascontrol)
    (Pawn|Input|AddMovementInput (Variables|Default|GetPlayer%20reference) (Math|Vector|MakeVector 0.0 (* AxisValue (Variables|Default|GetInput%20speed)) 0.0) 1.0 false)))

(fn ConstructionScript)