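; Tombstone level actor that acts as a grave interaction zone for the BP_JohnCena player character.
; Entering its box trigger shows a widget component and sets the player's Isatgrave flag; leaving hides the widget and clears the flag.
; The overlap handlers check the controlled pawn of player 0 rather than the overlapping actor.
; Separately, 30 seconds after BeginPlay it fades in a piano solo audio component.
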(event OnComponentBeginOverlap(Box)
  (params (OtherActor :type Actor%20Object%20Reference) (OtherComp :type Primitive%20Component%20Object%20Reference) (OtherBodyIndex :type Integer) (bFromSweep :type Boolean) (SweepResult :type Hit%20Result%20Structure%20%28by%20ref%29))
  (bind _asbp_john_cena (Utilities|Casting|CastToBP_JohnCena (Pawn|GetControlledPawn (Game|GetPlayerController 0))))
  (Development|SetHiddeninGame (Variables|Default|GetWidget) false false)
  (Variables|/Game/Derzo/Minigame1/JohnCena/BP_JohnCena.BP_JohnCena_C|Setisatgrave _asbp_john_cena true))

(event OnComponentEndOverlap(Box)
  (params (OtherActor :type Actor%20Object%20Reference) (OtherComp :type Primitive%20Component%20Object%20Reference) (OtherBodyIndex :type Integer))
  (Development|SetHiddeninGame (Variables|Default|GetWidget) true false)
  (bind _asbp_john_cena (Utilities|Casting|CastToBP_JohnCena (Pawn|GetControlledPawn (Game|GetPlayerController 0))))
  (Variables|/Game/Derzo/Minigame1/JohnCena/BP_JohnCena.BP_JohnCena_C|Setisatgrave _asbp_john_cena false))

(event EventBeginPlay
  (Utilities|FlowControl|Delay 3e+01)
  (Audio|Components|Audio|FadeIn (Variables|Default|GetPiano_Solo__1_RF) 1.0 1.0 0.0 :!class /Script/Engine.AudioComponent))

(event EventActorBeginOverlap
  (params (OtherActor :type Actor%20Object%20Reference)))

(event EventTick
  (params (DeltaSeconds :type Float%20%28single-precision%29)))

(fn ConstructionScript)